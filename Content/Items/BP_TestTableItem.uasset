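; BP_TestTableItem is a test item actor that fades in as it animates a drop through an approach point to a final position.
; BeginPlay makes a dynamic material on the mesh and hides it through the Opacity parameter.
; StartDrop stores both targets, then one timeline drives two chained lerps split at 0.7, raising opacity only during the first leg.
; A separate slide timeline is left unconnected.
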(event Custom|StartDrop
  (params (ApproachTarget%20%20%20 :type Vector) (FinalTarget :type Vector))
  (CallFunction|StartTableDrop ApproachTarget%20%20%20 FinalTarget)
  (bind _dropalpha (Timeline|TL_TableDrop PlayFromStart)
    (:Update
      (if (< _dropalpha 0.7)
        (Transformation|SetActorLocation (Math|Vector|Lerp(Vector) (Variables|Default|GetStartLocation) (Variables|Default|GetTargetLocation) (Math|Float|MapRangeClamped _dropalpha 0.0 0.7 0.0 1.0)) false false)
        (Rendering|Material|SetScalarParameterValue (Variables|Default|GetItemDynamicMaterial) "Opacity" _dropalpha :!class /Script/Engine.MaterialInstanceDynamic)
        (else
          (Transformation|SetActorLocation (Math|Vector|Lerp(Vector) (Variables|Default|GetTargetLocation) (Variables|Default|GetFinalTargetLocation) (Math|Float|MapRangeClamped _dropalpha 0.7 1.0 0.0 1.0)) false false))))))

(event EventBeginPlay
  (bind _returnvalue (Rendering|Material|CreateDynamicMaterialInstance (Variables|Default|GetItemMesh) 0 0 "None" :!class /Script/Engine.PrimitiveComponent))
  (bind _output_get (Variables|Default|SetItemDynamicMaterial _returnvalue))
  (Rendering|Material|SetScalarParameterValue _output_get "Opacity" 0.0 :!class /Script/Engine.MaterialInstanceDynamic))

(fn ConstructionScript)

(fn StartTableDrop
  (params (ApproachTarget :type Vector) (FinalTarget :type Vector))
  (Variables|Default|SetStartLocation (Transformation|GetActorLocation))
  (Variables|Default|SetTargetLocation ApproachTarget)
  (Variables|Default|SetFinalTargetLocation FinalTarget))