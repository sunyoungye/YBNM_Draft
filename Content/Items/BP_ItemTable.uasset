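; BP_ItemTable is an interactable table that lets the first-person player inspect items dropped onto it.
; Inside its box, a per-tick look-direction dot product toggles the interact prompt, and overlap registers the table on the character.
; Enter/Exit events blend the camera between table and player, switching cursor and input mode.
; BeginPlay spawns three staggered test items that drop toward the first free slot; SelectItem is an empty stub.
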(event OnComponentBeginOverlap(Box)
  (params (OverlappedComponent :type Primitive%20Component%20Object%20Reference) (OtherActor :type Actor%20Object%20Reference) (OtherComp :type Primitive%20Component%20Object%20Reference) (OtherBodyIndex :type Integer) (bFromSweep :type Boolean) (SweepResult :type Hit%20Result%20Structure%20%28by%20ref%29))
  ;[0.15 0.003193 0 0.5] CAPTION | When hit the box collision
  (bind _asbp_first_person_character (Utilities|Casting|CastToBP_FirstPersonCharacter OtherActor))
  (Variables|Default|SetOverlappingPlayer _asbp_first_person_character)
  (Variables|/Game/FirstPerson/Blueprints/BP_FirstPersonCharacter.BP_FirstPersonCharacter_C|SetCurrentItemTable _asbp_first_person_character self)
  (Variables|Default|SetPlayerInside true))

(event OnComponentEndOverlap(Box)
  (params (OverlappedComponent :type Primitive%20Component%20Object%20Reference) (OtherActor :type Actor%20Object%20Reference) (OtherComp :type Primitive%20Component%20Object%20Reference) (OtherBodyIndex :type Integer))
  ;[0.15 0.003193 0 0.5] CAPTION | When hit the box collision
  (bind _asbp_first_person_character (Utilities|Casting|CastToBP_FirstPersonCharacter OtherActor))
  (Variables|/Game/FirstPerson/Blueprints/BP_FirstPersonCharacter.BP_FirstPersonCharacter_C|SetCurrentItemTable _asbp_first_person_character 0)
  (Variables|Default|SetPlayerInside false)
  (Variables|Default|SetOverlappingPlayer 0)
  (CallFunction|HideInteract))

(event Custom|EnterTableView
  (bind _returnvalue (Game|GetPlayerController 0))
  (Game|Player|SetViewTargetwithBlend _returnvalue self 0.4 "VTBlend_Linear" 0.0 false)
  (Variables|/Script/Engine.PlayerController|SetbShowMouseCursor _returnvalue true)
  (Variables|/Script/Engine.PlayerController|SetbEnableMouseOverEvents _returnvalue true)
  (Input|SetInputModeGameandUI _returnvalue 0 "DoNotLock" true false))

(event Custom|ExitTableView
  (bind _returnvalue (Game|GetPlayerController 0))
  (Game|Player|SetViewTargetwithBlend _returnvalue (Game|GetPlayerCharacter 0) 0.4 "VTBlend_Linear" 0.0 false)
  (Variables|/Script/Engine.PlayerController|SetbShowMouseCursor _returnvalue false)
  (Variables|/Script/Engine.PlayerController|SetbEnableMouseOverEvents _returnvalue false)
  (Input|SetInputModeGameOnly _returnvalue false)
  (Input|SetIgnoreMoveInput _returnvalue false)
  (Input|SetIgnoreLookInput _returnvalue false))

(event Custom|SelectItem
  (params (NewItem :type BP%20Test%20Table%20Item%20Object%20Reference)))

(event Custom|HideInteract
  (bind _interactwidget (Variables|Default|GetInteractWidget))
  ;[0.15 0.007152 0 0.5] CAPTION | Show Interact & Hide Interact
  (if (Utilities|IsValid _interactwidget)
    (Widget|RemovefromParent _interactwidget)))

(event Custom|ShowInteract
  ;[0.15 0.007152 0 0.5] CAPTION | Show Interact & Hide Interact
  (if (Utilities|IsValid (Variables|Default|GetInteractWidget))
    (if (not (UserInterface|Viewport|IsinViewport (Variables|Default|GetInteractWidget)))
      (UserInterface|Viewport|AddtoViewport (Variables|Default|GetInteractWidget) 0)
      (Default|UpdateText (Variables|Default|GetInteractWidget) "[E] Inspect Items"))
    (else
      (bind _returnvalue (UserInterface|CreateWidget "/Game/UI/WBP_Interact.WBP_Interact_C" (Game|GetPlayerController 0)))
      (bind _output_get (Variables|Default|SetInteractWidget _returnvalue))
      (UserInterface|Viewport|AddtoViewport _output_get 0)
      (Default|UpdateText (Variables|Default|GetInteractWidget) "[E] Inspect Items"))))

(event EventBeginPlay
  (UserInterface|CreateWidget "/Game/UI/WBP_Interact.WBP_Interact_C" (Game|GetPlayerController 0))
  (CallFunction|SpawnTestItem "/Game/Items/BP_TestTableItem.BP_TestTableItem_C")
  (Utilities|FlowControl|Delay 2.2)
  (CallFunction|SpawnTestItem "/Game/Items/BP_TestTableItem.BP_TestTableItem_C")
  (Utilities|FlowControl|Delay 2.2)
  (CallFunction|SpawnTestItem "/Game/Items/BP_TestTableItem.BP_TestTableItem_C"))

(event EventTick
  (params (DeltaSeconds :type Float%20%28single-precision%29))
  (bind _overlappingplayer (Variables|Default|GetOverlappingPlayer))
  (bind _firstpersoncamera (Variables|/Game/FirstPerson/Blueprints/BP_FirstPersonCharacter.BP_FirstPersonCharacter_C|GetFirstPersonCamera _overlappingplayer))
  ;[0.15 0.003929 0 0.5] CAPTION
  (if (Variables|Default|GetPlayerInside)
    (if (> (Math|Vector|DotProduct (Math|Vector|GetForwardVector _firstpersoncamera) (Math|Vector|GetUnitDirection(Vector) (Transformation|GetWorldLocation _firstpersoncamera) (Transformation|GetWorldLocation (Variables|Default|GetInteractLookPoint)))) 0.9)
      (CallFunction|ShowInteract)
      (else
        (CallFunction|HideInteract)))))

(fn ConstructionScript)

(fn SpawnTestItem
  (params (ItemClass :type BP%20Test%20Table%20Item%20Class%20Reference))
  (bind _droppoint (Variables|Default|GetDropPoint))
  (bind _itemslot_01 (Variables|Default|GetItemSlot_01))
  (bind _returnvalue (Transformation|GetWorldTransform _droppoint))
  (bind _returnvalue_2 (Transformation|GetWorldLocation _itemslot_01))
  (if (Utilities|IsValid (Variables|Default|GetSlot1Item))
    (if (Utilities|IsValid (Variables|Default|GetSlot2Item))
      (if (Utilities|IsValid (Variables|Default|GetSlot3Item))
        (Development|PrintString "Table Full")
        (else
          (bind _returnvalue_3 (Game|SpawnActorfromClass "/Game/Items/BP_TestTableItem.BP_TestTableItem_C" _returnvalue "AlwaysSpawn" "MultiplyWithRoot" 0 0))
          (Variables|/Game/Items/BP_TestTableItem.BP_TestTableItem_C|SetOwnerTable _returnvalue_3 self)
          (bind _output_get (Variables|Default|SetSlot3Item _returnvalue_3))
          (Default|StartDrop _output_get (Transformation|GetWorldLocation (Variables|Default|GetSlidePoint)) (Transformation|GetWorldLocation (Variables|Default|GetItemSlot_03)))))
      (else
        (bind _returnvalue_4 (Game|SpawnActorfromClass "/Game/Items/BP_TestTableItem.BP_TestTableItem_C" _returnvalue "AlwaysSpawn" "MultiplyWithRoot" 0 0))
        (Variables|/Game/Items/BP_TestTableItem.BP_TestTableItem_C|SetOwnerTable _returnvalue_4 self)
        (bind _output_get_2 (Variables|Default|SetSlot2Item _returnvalue_4))
        (Default|StartDrop _output_get_2 (Transformation|GetWorldLocation (Variables|Default|GetSlidePoint)) (Transformation|GetWorldLocation (Variables|Default|GetItemSlot_02)))))
    (else
      (bind _returnvalue_5 (Game|SpawnActorfromClass "/Game/Items/BP_TestTableItem.BP_TestTableItem_C" _returnvalue "AlwaysSpawn" "MultiplyWithRoot" 0 0))
      (Variables|/Game/Items/BP_TestTableItem.BP_TestTableItem_C|SetOwnerTable _returnvalue_5 self)
      (bind _output_get_3 (Variables|Default|SetSlot1Item _returnvalue_5))
      (Default|StartDrop _output_get_3 _returnvalue_2 _returnvalue_2))))