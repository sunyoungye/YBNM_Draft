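; Arcade machine actor that registers itself as the first-person character's CurrentMachine while that character overlaps its collider.
; StartSpin snaps the player to a stand point and plays a timeline that turns the Rotator component through a full yaw revolution, until StopSpin halts it.
; A second timeline lerps the spring arm length for camera zoom and reverses to undo it.
; Spin and zoom are events with no callers in this Blueprint.
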(event OnComponentBeginOverlap(Collider)
  (params (OverlappedComponent :type Primitive%20Component%20Object%20Reference) (OtherActor :type Actor%20Object%20Reference) (OtherComp :type Primitive%20Component%20Object%20Reference) (OtherBodyIndex :type Integer) (bFromSweep :type Boolean) (SweepResult :type Hit%20Result%20Structure%20%28by%20ref%29))
  (bind _asbp_first_person_character (Utilities|Casting|CastToBP_FirstPersonCharacter OtherActor))
  (Variables|/Game/FirstPerson/Blueprints/BP_FirstPersonCharacter.BP_FirstPersonCharacter_C|SetCurrentMachine _asbp_first_person_character self))

(event OnComponentEndOverlap(Collider)
  (params (OverlappedComponent :type Primitive%20Component%20Object%20Reference) (OtherActor :type Actor%20Object%20Reference) (OtherComp :type Primitive%20Component%20Object%20Reference) (OtherBodyIndex :type Integer))
  (bind _asbp_first_person_character (Utilities|Casting|CastToBP_FirstPersonCharacter OtherActor))
  (Variables|/Game/FirstPerson/Blueprints/BP_FirstPersonCharacter.BP_FirstPersonCharacter_C|SetCurrentMachine _asbp_first_person_character 0))

(event Custom|StartSpin
  (bind _playerstandpoint (Variables|Default|GetPlayerStandPoint))
  (Transformation|SetActorLocationAndRotation (Game|GetPlayerCharacter 0) (Transformation|GetWorldLocation _playerstandpoint) (Transformation|GetWorldRotation _playerstandpoint))
  (bind _alpha (Timeline|Timeline Play)
    (:Update
      (Transformation|SetRelativeRotation (Variables|Default|GetRotator) (Math|Rotator|MakeRotator 0.0 0.0 (Math|Float|Lerp 0.0 3.6e+02 _alpha)) false false))))

(event Custom|StopSpin
  (bind _alpha (Timeline|Timeline Stop)
    (:Update
      (Transformation|SetRelativeRotation (Variables|Default|GetRotator) (Math|Rotator|MakeRotator 0.0 0.0 (Math|Float|Lerp 0.0 3.6e+02 _alpha)) false false))))

(event Custom|CameraZoom
  (bind _alpha (Timeline|ZoomAnim Play)
    (:Update
      (Variables|/Script/Engine.SpringArmComponent|SetTargetArmLength (Variables|Default|GetSpringArm) (Math|Float|Lerp (Variables|Default|GetDefaultArmLength) (Variables|Default|GetZoomArmLength) _alpha)))))

(event Custom|CameraZoomReverse
  (bind _alpha (Timeline|ZoomAnim Reverse)
    (:Update
      (Variables|/Script/Engine.SpringArmComponent|SetTargetArmLength (Variables|Default|GetSpringArm) (Math|Float|Lerp (Variables|Default|GetDefaultArmLength) (Variables|Default|GetZoomArmLength) _alpha)))))

(event EventBeginPlay)

(event Collision|EventActorBeginOverlap
  (params (OtherActor :type Actor%20Object%20Reference)))

(event EventTick
  (params (DeltaSeconds :type Float%20%28single-precision%29)))

(fn ConstructionScript)