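; Day manager that runs the game's timed day cycle, granting the player a token at each day start.
; BeginPlay creates the day HUD, hands it to the character, starts the day and lowers screen percentage.
; A looping one-second timer drives the countdown; EndDay, guarded against repeats, pauses the game and shows a report widget holding a manager reference.
; AdvanceDay increments the day and restarts the cycle.
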(event Custom|EndDay
  (bind _returnvalue (Game|GetPlayerController 0))
  ;[0.15 2.9e-05 0.00354 0.5] Make Report Pop Up
  (if (not (Variables|Default|GetIsDayEnding))
    (Variables|Default|SetIsDayEnding true)
    (Utilities|Time|ClearandInvalidateTimerbyHandle (Variables|Default|GetDayTimerHandle))
    (bind _returnvalue_2 (UserInterface|CreateWidget "/Game/DaySystem/WBP_DayReport.WBP_DayReport_C" 0 (Variables|Default|GetCurrentDay) self))
    (UserInterface|Viewport|AddtoViewport _returnvalue_2 0)
    (Variables|/Script/Engine.PlayerController|SetbShowMouseCursor _returnvalue true)
    (Input|SetInputModeUIOnly _returnvalue 0 "DoNotLock" false)
    (Game|SetGamePaused true)))

(event Custom|AdvanceDay
  ;[0.15 0 0.003677 0.502] Make Day Pass(?)
  (Variables|Default|SetCurrentDay (+ (Variables|Default|GetCurrentDay) 1))
  (CallFunction|StartDay))

(event Custom|StartDay
  ;[0.15 0.15 0.15 0.5] Start Day
  (Variables|Default|SetTimeRemaining (Variables|Default|GetDayDuration))
  (Variables|Default|SetIsDayEnding false)
  (bind _returnvalue (Utilities|Time|SetTimerbyEvent (EventDispatchers|CreateEvent :!event Custom|UpdateDayTimer) 1.0 true))
  (Variables|Default|SetDayTimerHandle _returnvalue)
  (bind _asbp_first_person_character (Utilities|Casting|CastToBP_FirstPersonCharacter (Game|GetPlayerCharacter 0)))
  (Default|AddToken _asbp_first_person_character 1))

(event Custom|UpdateDayTimer
  ;[0.15 0.15 0.15 0.5] Update Day Timer
  (bind _output_get (Variables|Default|SetTimeRemaining (- (Variables|Default|GetTimeRemaining) 1.0)))
  (Development|PrintString (Utilities|String|ToString(Float) (Variables|Default|GetTimeRemaining)) true true "(R=0.000000,G=0.660000,B=1.000000,A=1.000000)" 0.9)
  (if (<= _output_get 0.0)
    (CallFunction|EndDay)))

(event EventBeginPlay
  (bind _returnvalue (UserInterface|CreateWidget "/Game/DaySystem/WBP_DayHUD.WBP_DayHUD_C"))
  (UserInterface|Viewport|AddtoViewport _returnvalue 0)
  (bind _asbp_first_person_character (Utilities|Casting|CastToBP_FirstPersonCharacter (Game|GetPlayerCharacter 0)))
  (Variables|/Game/FirstPerson/Blueprints/BP_FirstPersonCharacter.BP_FirstPersonCharacter_C|SetHUDRef _asbp_first_person_character _returnvalue)
  (CallFunction|StartDay)
  (Development|ExecuteConsoleCommand "r.ScreenPercentage 35" 0))

(fn ConstructionScript)